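; BombBP is a bomb Blueprint that can be switched on and off during gameplay.
; On BeginPlay it caches a reference to the GameplayGM game mode.
; EnableBombEvent toggles the particle system, resetting it, and adds or removes the bomb from the game mode's ActiveBombs collection, so the game mode tracks which bombs are live.
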(event `self.ReceiveBeginPlay`
  (bind _asgameplay_gm (cast `/Game/Blueprint/GameplayGM` (`GameplayStatics.GetGameMode`)))
  (set `self.GMRef` _asgameplay_gm))

(event `self.EnableBombEvent`
  (params (enabled :type Boolean))
  (bind _gmref (`self.GMRef`))
  (`ActorComponent.SetActive` (`self.ParticleSystem`) enabled true)
  (`/Engine/EditorBlueprintResources/StandardMacros.IsValid` (`self.GMRef`)
    (:`Is Valid`
      (if enabled
        (`KismetArrayLibrary.Array_Add` (`/Game/Blueprint/GameplayGM.ActiveBombs` _gmref) self)
        (else
          (`KismetArrayLibrary.Array_RemoveItem` (`/Game/Blueprint/GameplayGM.ActiveBombs` _gmref) self))))))

(fn `UserConstructionScript`)