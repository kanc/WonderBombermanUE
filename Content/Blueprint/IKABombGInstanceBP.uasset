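; Game instance for IKABomb that owns saved game history, graphics settings and level travel between the menu and maps.
; On Init it shows the intro widget, loads or creates both save files, applies settings and clears a main-menu wait flag after a delay.
; Detail level selects a Low, Mid or High template for GameUserSettings, with resolution changed only when different.
; Starting a game fades the screen and opens a chosen or random map, falling back to the menu.
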(event `SaveGameData`
  (params (lastGame :type "/Game/Data/GamesData Structure"))
  (`KismetArrayLibrary.Array_Add` (`/Game/Data/SaveGameFile.GamesList` (`self.SavedGamesFile`)) lastGame)
  (`GameplayStatics.SaveGameToSlot` (`self.SavedGamesFile`) (`self.SavedGameSlotName`)))

(event `LoadGameData`
  (bind _returnvalue (`GameplayStatics.DoesSaveGameExist` (`self.SavedGameSlotName`)))
  (if _returnvalue
    (bind _returnvalue_2 (`GameplayStatics.LoadGameFromSlot` (`self.SavedGameSlotName`)))
    (bind _assave_game_file (cast `/Game/Data/SaveGameFile` _returnvalue_2))
    (set `self.SavedGamesFile` _assave_game_file)
    (else
      (bind _returnvalue_3 (`GameplayStatics.CreateSaveGameObject` "/Game/Data/SaveGameFile.SaveGameFile_C"))
      (set `self.SavedGamesFile` _returnvalue_3))))

(event `self.ReceiveInit`
  (bind _returnvalue (`|CreateWidget` "/Game/UI/UIIntro_W.UIIntro_W_C"))
  (`UserWidget.AddToViewport` _returnvalue 0)
  (`self.LoadAndApplySettings`)
  (`self.LoadGameData`)
  (`KismetSystemLibrary.Delay` 2.5)
  (set `self.WaitForMainMenu` false))

(event `FadeAndStartGame`
  (bind (_value _returnvalue) (`BlueprintMapLibrary.Map_Find` (`self.Maps`) (`self.MapType`)))
  (`PlayerCameraManager.StartCameraFade` (`GameplayStatics.GetPlayerCameraManager` 0) 0.0 1.0 2.0 (struct :`R` 1.0 :`G` 1.0 :`B` 1.0 :`A` 1.0) true true)
  (`KismetSystemLibrary.Delay` 2.1)
  (if (`self.AutoMap`)
    (set `self.MapType` (cast `EMapType` (`KismetMathLibrary.Conv_IntToByte` (`KismetMathLibrary.RandomIntegerInRange` 0 (- (`BlueprintMapLibrary.Map_Length` (`self.Maps`)) 1))))))
  (if _returnvalue
    (`GameplayStatics.OpenLevel` (`KismetStringLibrary.Conv_StringToName` _value))
    (else
      (`GameplayStatics.OpenLevel` (`self.MenuMap`)))))

(event `RestartGame`
  (params (restart :type Boolean))
  (bind (_value _returnvalue) (`BlueprintMapLibrary.Map_Find` (`self.Maps`) (`self.MapType`)))
  (if (and _returnvalue restart)
    (`GameplayStatics.OpenLevel` (`KismetStringLibrary.Conv_StringToName` _value))
    (else
      (`GameplayStatics.OpenLevel` (`self.MenuMap`)))))

(event `SetSettings`
  (params (level :type Integer) (Width :type Integer) (Height :type Integer))
  (set `/Game/Data/SaveSettingsFile.Settings` (make `/Game/Data/SettingsData` level Width Height) (`self.SettingsFile`))
  (`self.SaveDetails`))

(event `SaveDetails`
  (`GameplayStatics.SaveGameToSlot` (`self.SettingsFile`) (`self.SettingsSlotName`)))

(event `LoadAndApplySettings`
  (bind _returnvalue (`GameplayStatics.DoesSaveGameExist` (`self.SettingsSlotName`)))
  (if _returnvalue
    (bind _returnvalue_2 (`GameplayStatics.LoadGameFromSlot` (`self.SettingsSlotName`)))
    (bind _assave_settings_file (cast `/Game/Data/SaveSettingsFile` _returnvalue_2))
    (set `self.SettingsFile` _assave_settings_file)
    (else
      (bind _returnvalue_3 (`GameplayStatics.CreateSaveGameObject` "/Game/Data/SaveSettingsFile.SaveSettingsFile_C"))
      (set `self.SettingsFile` _returnvalue_3)))
  (`self.ApplyCurrentSettings`))

(event `ApplyCurrentSettings`
  (switch `int` (`.DetailLevel_2_3305F25A41AC45F5802BDBA2BC062B9A` (break `/Game/Data/SettingsData` (`/Game/Data/SaveSettingsFile.Settings` (`self.SettingsFile`))))
    (:`Default`
      (`self.ApplySettings` (`self.HighSettingsTemplate`) :!label _label))
    (:`0`
      (`self.ApplySettings` (`self.LowSettingsTemplate`)))
    (:`1`
      (`self.ApplySettings` (`self.MidSettingsTemplate`)))
    (:`2`
      (goto _label))))

(fn `ApplySettings`
  (params (settings :type "/Game/Data/DetailSettings Structure"))
  (bind (_shadow _texture _visualdist _effects _aa _pp _foliage) (break `/Game/Data/DetailSettings` settings))
  (bind (_detaillevel _reswidth _resheight) (break `/Game/Data/SettingsData` (`/Game/Data/SaveSettingsFile.Settings` (`self.SettingsFile`))))
  (bind (_detaillevel_2 _reswidth_2 _resheight_2) (break `/Game/Data/SettingsData` (`/Game/Data/SaveSettingsFile.Settings` (`self.SettingsFile`))))
  (bind _returnvalue (`GameUserSettings.GetGameUserSettings`))
  (`|ExecutionSequence`
    (:`then_0`
      (`GameUserSettings.SetViewDistanceQuality` _returnvalue _visualdist)
      (`GameUserSettings.SetShadowQuality` _returnvalue _shadow))
    (:`then_1`
      (`GameUserSettings.SetTextureQuality` _returnvalue _texture)
      (`GameUserSettings.SetVisualEffectQuality` _returnvalue _effects))
    (:`then_2`
      (`GameUserSettings.SetAntiAliasingQuality` _returnvalue _aa)
      (`GameUserSettings.SetPostProcessingQuality` _returnvalue _pp)
      (`GameUserSettings.SetFoliageQuality` _returnvalue _foliage))
    (:`then_3`
      (`GameUserSettings.ApplyNonResolutionSettings` _returnvalue)
      (bind (_x _y) (break `IntPoint` (`GameUserSettings.GetScreenResolution` _returnvalue)))
      (if (or (!= _reswidth_2 _x) (!= _resheight_2 _y))
        (`GameUserSettings.SetScreenResolution` _returnvalue (make `IntPoint` _reswidth _resheight))
        (`KismetSystemLibrary.ExecuteConsoleCommand` (`KismetStringLibrary.Concat_StrStr` "r.SetRes " (`KismetStringLibrary.Conv_IntToString` _reswidth) "x" (`KismetStringLibrary.Conv_IntToString` _resheight) "f"))))))