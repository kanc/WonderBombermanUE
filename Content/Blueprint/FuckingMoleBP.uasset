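; Mole hazard actor that periodically pops out of the ground to steal pickups or, when none exist, active bombs.
; A randomized timer calls StoleItem, which rolls a probability, picks a random IKAPickup actor or bomb from GameplayGM's ActiveBombs, and removes it.
; The mole teleports just below the stolen item, plays rise animation, smoke and sound, then retreats on a second timer.
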(event `self.ReceiveBeginPlay`
  (bind _asgameplay_gm (cast `/Game/Blueprint/GameplayGM` (`GameplayStatics.GetGameMode`)))
  (set `self.GMRef` _asgameplay_gm)
  (`KismetSystemLibrary.Delay` 2.0)
  (`self.NewStoleTry`))

(fn `GetDownMole`
  (`SkeletalMeshComponent.PlayAnimation` (`self.MoleMesh`) "/Game/Animations/MoleGetDown.MoleGetDown" false)
  (`ActorComponent.SetActive` (`self.SmokeGround`) true true)
  (`GameplayStatics.PlaySoundAtLocation` (`self.ActionSound`) (`self.K2_GetActorLocation`)))

(fn `GetUpMole`
  (params (Location :type "Vector Structure"))
  (`self.K2_SetActorLocation` (- Location (0.0 0.0 45.0)))
  (`SkeletalMeshComponent.PlayAnimation` (`self.MoleMesh`) "/Game/Animations/MoleGetUp.MoleGetUp" false)
  (`ActorComponent.SetActive` (`self.SmokeGround`) true true)
  (`GameplayStatics.PlaySoundAtLocation` (`self.ActionSound`) (`self.K2_GetActorLocation`))
  (`KismetSystemLibrary.K2_SetTimer` self "GetDownMole" (`self.TimeOutside`)))

(fn `NewStoleTry`
  (bind (_x _y) (`KismetMathLibrary.BreakVector2D` (`self.TimeToStole`)))
  (`KismetSystemLibrary.K2_SetTimer` self "StoleItem" (`KismetMathLibrary.RandomFloatInRange` _x _y)))

(fn `StoleItem`
  (locals (index :type Integer))
  (bind _gmref (`self.GMRef`))
  (bind _activebombs (`/Game/Blueprint/GameplayGM.ActiveBombs` _gmref))
  (bind _returnvalue (`KismetArrayLibrary.Array_Length` _activebombs))
  (bind _output (`|GetArrayItem` _activebombs (`local.index`)))
  (bind _returnvalue_2 (`IKABombUtils.CheckProbability` (`self.StolePercentage`)))
  (if _returnvalue_2
    ;[1 1 1] Stole Pickups
    (bind _outactors (`GameplayStatics.GetAllActorsOfClass` "/Script/IKABombermanUE.IKAPickup"))
    (bind _returnvalue_3 (`KismetArrayLibrary.Array_Length` _outactors))
    (if (> _returnvalue_3 0)
      (set `local.index` (`KismetMathLibrary.RandomIntegerInRange` 0 (- _returnvalue_3 1)))
      (bind _output_2 (`|GetArrayItem` _outactors (`local.index`)))
      (`self.GetUpMole` (`self.K2_GetActorLocation` _output_2))
      (`IKADestructibleObj.DestroyObj` _output_2)
      (`self.NewStoleTry`)
      (else
        ;[1 1 1] Stole bombs
        (`/Engine/EditorBlueprintResources/StandardMacros.IsValid` _gmref
          (:`Is Valid`
            (if (> _returnvalue 0)
              (set `local.index` (`KismetMathLibrary.RandomIntegerInRange` 0 (- _returnvalue 1)))
              (`self.GetUpMole` (`self.K2_GetActorLocation` _output))
              (`IKABomb.BombStolen` _output)
              (`self.NewStoleTry`)
              (else
                (`self.NewStoleTry`)))))))
    (else
      (`self.NewStoleTry`))))

(fn `UserConstructionScript`)