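; A projectile actor that flies in a straight line and deals point damage to what it hits.
; Tick moves it along MovDirection at Speed, scaled by delta time and without sweep, so hits rely on the Detector component's overlap.
; On overlap it applies damage to the other actor, spawns a blast particle effect and destroys itself.
; The DestroyProj function is an empty stub.
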(event `self.ReceiveTick`
  (params (DeltaSeconds :type "Float (single-precision)"))
  (`self.K2_SetActorLocation` (+ (`self.K2_GetActorLocation`) (* (`self.MovDirection`) (* (`self.Speed`) (`GameplayStatics.GetWorldDeltaSeconds`))))))

(event `self.Detector.OnComponentBeginOverlap`
  (params (OverlappedComponent :type "PrimitiveComponent Object Reference") (OtherActor :type "Actor Object Reference") (OtherComp :type "PrimitiveComponent Object Reference") (OtherBodyIndex :type Integer) (bFromSweep :type Boolean) (SweepResult :type "HitResult Structure (by ref)"))
  (`GameplayStatics.ApplyPointDamage` OtherActor 1.0 (`self.MovDirection`) SweepResult null self "/Script/Engine.DamageType")
  (`GameplayStatics.SpawnEmitterAtLocation` "/Game/FX/Blast_P.Blast_P" (`self.K2_GetActorLocation`))
  (`self.K2_DestroyActor`))

(fn `DestroyProj`)

(fn `UserConstructionScript`)