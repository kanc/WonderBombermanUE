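; Mummy enemy Character that appears at random navmesh points after a random delay, wanders, chases overlapping actors and deals point damage on contact.
; Timers drive EnableMummy, which respawns only during the game mode's playing state, then ShowMesh, which activates it.
; AIMoveTo completion loops between wandering and chasing the Sphere's target.
; Hits flash a pose-synced Fresnel mesh with brief invulnerability; death plays FX, hides it and reschedules its return.
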(event `self.ReceiveBeginPlay`
  (bind (_x _y) (`KismetMathLibrary.BreakVector2D` (`self.TimeRangeToAppear`)))
  (`SceneComponent.SetVisibility` (`self.Mesh`) false true)
  (`KismetSystemLibrary.K2_SetTimer` self "EnableMummy" (`KismetMathLibrary.RandomFloatInRange` _x _y)))

(event `GoTo`
  (params (delay :type "Float (double-precision)") (Location :type "Vector Structure"))
  (`KismetSystemLibrary.Delay` delay)
  (`AITask_MoveTo.AIMoveTo` (`AIBlueprintHelperLibrary.GetAIController` self) Location null 20.0 "Default" "Enable" true true true
    (:`then`
      (`KismetSystemLibrary.PrintString` "move"))
    (:`OnRequestFailed`
      (`self.NavigationFailed`))
    (:`OnMoveFinished`
      (`self.PointReached`))))

(event `ChasePlayer`
  (`AITask_MoveTo.AIMoveTo` (`AIBlueprintHelperLibrary.GetAIController` self) (0.0 0.0 0.0) (`self.Target`) 20.0 "Default" "Enable" true true true
    (:`then`
      (`KismetSystemLibrary.PrintString` "Chase " true true (struct :`G` 1.0 :`B` 0.033423 :`A` 1.0)))
    (:`OnRequestFailed`
      (`self.NavigationFailed`))
    (:`OnMoveFinished`
      (`self.PointReached`))))

(event `PointReached`
  (if (`self.Active`)
    (`/Engine/EditorBlueprintResources/StandardMacros.IsValid` (`self.Target`)
      (:`Is Valid`
        (`self.ChasePlayer`))
      (:`Is Not Valid`
        (`self.GetRandomTargetPoint`)))))

(event `NavigationFailed`)

(event `self.Sphere.OnComponentBeginOverlap`
  (params (OverlappedComponent :type "PrimitiveComponent Object Reference") (OtherActor :type "Actor Object Reference") (OtherComp :type "PrimitiveComponent Object Reference") (OtherBodyIndex :type Integer) (bFromSweep :type Boolean) (SweepResult :type "HitResult Structure (by ref)"))
  (if (`self.Active`)
    (`/Engine/EditorBlueprintResources/StandardMacros.IsValid` (`self.Target`)
      (:`Is Not Valid`
        (set `self.Target` OtherActor)
        (`MovementComponent.StopMovementImmediately` (`self.CharacterMovement`))
        (`self.ChasePlayer`)))))

(event `self.Sphere.OnComponentEndOverlap`
  (params (OverlappedComponent :type "PrimitiveComponent Object Reference") (OtherActor :type "Actor Object Reference") (OtherComp :type "PrimitiveComponent Object Reference") (OtherBodyIndex :type Integer))
  (if (== OtherActor (`self.Target`))
    (set `self.Target` null)))

(event `self.ReceivePointDamage`
  (params (Damage :type "Float (single-precision)") (DamageType :type "DamageType Object Reference") (HitLocation :type "Vector Structure") (HitNormal :type "Vector Structure") (HitComponent :type "PrimitiveComponent Object Reference") (BoneName :type Name) (ShotFromDirection :type "Vector Structure") (InstigatedBy :type "Controller Object Reference") (DamageCauser :type "Actor Object Reference") (HitInfo :type "HitResult Structure (by ref)"))
  (if (and (> (`self.Health`) 0.0) (`self.Active`))
    (set `self.bCanBeDamaged` false)
    (bind _result (`/Engine/EditorBlueprintResources/StandardMacros.DecrementFloat` (`self.Health`))
      (:`  `
        (if (<= _result 0.0)
          (`self.MummyDeath`)
          (`KismetSystemLibrary.PrintString` "death" true true (struct :`R` 1.0 :`B` 0.189691 :`A` 1.0))
          (else
            (`self.DamageMummy`)))))))

(event `MummyDeath`
  (bind (_x _y) (`KismetMathLibrary.BreakVector2D` (`self.TimeRangeToAppear`)))
  (set `self.Active` false)
  (set `CharacterMovementComponent.MaxWalkSpeed` 0.0 (`self.CharacterMovement`))
  (`KismetSystemLibrary.Delay` 2.0)
  (`ActorComponent.SetActive` (`self.DeathFX`) true true)
  (`SceneComponent.SetVisibility` (`self.Mesh`) false false)
  (`KismetSystemLibrary.Delay` 2.0)
  (`self.K2_SetActorLocation` (0.0 0.0 1000.0) false true)
  (`KismetSystemLibrary.K2_SetTimer` null "EnableMummy" (`KismetMathLibrary.RandomFloatInRange` _x _y)))

(event `self.DamageDealer.OnComponentBeginOverlap`
  (params (OverlappedComponent :type "PrimitiveComponent Object Reference") (OtherActor :type "Actor Object Reference") (OtherComp :type "PrimitiveComponent Object Reference") (OtherBodyIndex :type Integer) (bFromSweep :type Boolean) (SweepResult :type "HitResult Structure (by ref)"))
  (if (`self.Active`)
    (`GameplayStatics.ApplyPointDamage` OtherActor 1.0 (`self.GetActorForwardVector`) SweepResult (`AIBlueprintHelperLibrary.GetAIController` self) self)
    (`GameplayStatics.PlaySoundAtLocation` "/Game/Sound/MummyLaught.MummyLaught" (`self.K2_GetActorLocation`) (struct) 1.0 1.0 0.0 null null null)))

(fn `DamageMummy`
  (`SceneComponent.SetVisibility` (`self.FresnelMesh`) true false)
  (`KismetSystemLibrary.K2_SetTimer` self "HideFresnelMesh" (`self.DamageTime`))
  (`self.PlayAnimMontage` (`self.DamageMontage`)))

(fn `EnableMummy`
  (bind _asikagame_mode_base (cast `IKAGameModeBase` (`GameplayStatics.GetGameMode`)))
  (bind _returnvalue (`IKAGameModeBase.GetGameplayState` _asikagame_mode_base))
  (if (`|EnumEquality` _returnvalue "EPlaying")
    (set `self.Health` 2.0)
    (set `CharacterMovementComponent.MaxWalkSpeed` 100.0 (`self.CharacterMovement`))
    (`self.GetInitialSpawn`)))

(fn `GetInitialSpawn`
  (if true
    (`self.K2_SetActorLocation` (+ (`NavigationSystemV1.K2_GetRandomReachablePointInRadius` (`KismetMathLibrary.MakeVector` 0.0) (`self.RadiusToGetNavPoint`) null null) (`KismetMathLibrary.MakeVector` 0.0 0.0 (`self.HeightOffset`))) false true)
    (`ActorComponent.SetActive` (`self.SpawnFX`) true true)
    (`GameplayStatics.PlaySoundAtLocation` "/Game/Sound/MummyAppear.MummyAppear" (`self.K2_GetActorLocation`) (struct) 1.0 1.0 0.0 null null null)
    (`KismetSystemLibrary.K2_SetTimer` self "ShowMesh" (`self.DelayToShowMesh`))))

(fn `GetRandomTargetPoint`
  (bind (_randomlocation _returnvalue) (`NavigationSystemV1.K2_GetRandomReachablePointInRadius` (`self.K2_GetActorLocation`) (`self.RadiusToGetNavPoint`) null null))
  (if _returnvalue
    (`self.GoTo` 0.5 _randomlocation)
    (else
      (`KismetSystemLibrary.PrintString` "no point"))))

(fn `HideFresnelMesh`
  (`SceneComponent.SetVisibility` (`self.FresnelMesh`) false false)
  (set `self.bCanBeDamaged` true))

(fn `ShowMesh`
  (`SceneComponent.SetVisibility` (`self.Mesh`) true true)
  (set `self.Active` true)
  (`self.GetRandomTargetPoint`)
  (set `self.bCanBeDamaged` true)
  (`GameplayStatics.PlaySoundAtLocation` "/Game/Sound/MummyLaught.MummyLaught" (`self.K2_GetActorLocation`) (struct) 1.0 1.0 0.0 null null null))

(fn `UserConstructionScript`
  (`SkinnedMeshComponent.SetLeaderPoseComponent` (`self.FresnelMesh`) (`self.Mesh`) false))