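; Base player Blueprint that handles the remote-bomb indicator and the in-game pause menu.
; On BeginPlay it binds to the player UI update event and shows the RemoteBombImg component while the ERemoteBombs value is above zero.
; The pause event reuses the UIEndGame_W widget with its resume button enabled.
; Unpausing removes that widget, restores game-only input and hides the cursor.
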(event `self.ReceiveBeginPlay`
  (add `self.OnUpdatePlayerUI` (delegate `ShowRemote`)))

(event `ShowRemote` :!signature `self.OnUpdatePlayerUI`
  (params (PlayerProperty :type "EPlayerProperty Enum" :default "ESpeed") (value :type Integer))
  (if (`|EnumEquality` PlayerProperty "ERemoteBombs")
    (`SceneComponent.SetVisibility` (`self.RemoteBombImg`) (> value 0) false)))

(event `self.PauseGameBPEvent`
  (params (paused :type Boolean))
  (bind _returnvalue (`GameplayStatics.GetPlayerController` 0))
  (bind _ingamepausewidget (`self.InGamePauseWidget`))
  (if paused
    (bind _returnvalue_2 (`|CreateWidget` "/Game/UI/UIEndGame_W.UIEndGame_W_C"))
    (bind _output_get (set `self.InGamePauseWidget` _returnvalue_2))
    (`/Game/UI/UIEndGame_W.EnableResumeButton` _output_get)
    (`UserWidget.AddToViewport` _output_get 0)
    (else
      (`/Engine/EditorBlueprintResources/StandardMacros.IsValid` _ingamepausewidget
        (:`Is Valid`
          (`Widget.RemoveFromParent` _ingamepausewidget)
          (set `self.InGamePauseWidget` null)
          (`WidgetBlueprintLibrary.SetInputMode_GameOnly` _returnvalue)
          (set `PlayerController.bShowMouseCursor` false _returnvalue))))))

(fn `UserConstructionScript`)