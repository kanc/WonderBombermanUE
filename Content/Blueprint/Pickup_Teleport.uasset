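; Teleport pickup that swaps the collecting player's location with that of another player.
; PickupAction finds the collector in the GameplayGM game mode's CurrentPlayers array and selects the next entry, wrapping to the first.
; It caches the collector's location, then sends both players a SwapLocationMessage with the other's position.
; Teleport particles spawn at the collector's current and cached locations, and a slide sound plays at the world origin.
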(event `self.PickupAction`
  (params (actor :type "Actor Object Reference"))
  (bind _returnvalue (`self.K2_GetActorLocation` actor))
  (bind _location (`self.Location`))
  (bind _asgameplay_gm (cast `/Game/Blueprint/GameplayGM` (`GameplayStatics.GetGameMode`)))
  (bind _currentplayers (`IKAGameModeBase.CurrentPlayers` _asgameplay_gm))
  (for (_array_element _array_index) _currentplayers
    (if (== _array_element actor)
      (bind _output_get (set `self.IndexToSwap` (+ _array_index 1)))
      (if (== _output_get (`KismetArrayLibrary.Array_Length` _currentplayers))
        (set `self.IndexToSwap` 0)
        (break)
        (else
          (break)))))
  (set `self.Location` _returnvalue)
  (bind _output (`|GetArrayItem` _currentplayers (`self.IndexToSwap`)))
  (message `IKACanPickup.SwapLocation` actor (`self.K2_GetActorLocation` _output))
  (message `IKACanPickup.SwapLocation` _output _location)
  (`GameplayStatics.SpawnEmitterAtLocation` "/Game/FX/Teleport_P.Teleport_P" _returnvalue)
  (`GameplayStatics.SpawnEmitterAtLocation` "/Game/FX/Teleport_P.Teleport_P" _location)
  (`GameplayStatics.PlaySoundAtLocation` "/Game/Sound/slideSound.slideSound"))

(fn `UserConstructionScript`)