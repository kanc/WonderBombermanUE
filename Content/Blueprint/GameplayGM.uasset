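; Game mode for a local two-player bomb match, running it from map creation to the end-game menu.
; MapReady spawns and possesses both characters, starts the shared camera, builds the HUD and fades in, with input locked until GameStarted.
; A short timer after the first death detects same-causer draws; time-outs also draw, and results save through the game instance.
; Helpers handle restart/exit and temporary blackouts of level lights and post-processing.
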(event `self.ReceiveBeginPlay`
  (`PlayerCameraManager.StartCameraFade` (`GameplayStatics.GetPlayerCameraManager` 0) 0.0 1.0 0.001 (struct :`R` 1.0 :`G` 1.0 :`B` 1.0 :`A` 1.0) false true)
  (`parent.ReceiveBeginPlay`))

(event `self.MapReady`
  (bind _playersclass (`self.PlayersClass`))
  ;[1 1 1] Triggered when Map is created
  (`|ExecutionSequence`
    (:`then_0`
      ;[1 1 1] Get Camera Reference, create extra player. Spawn player characters, locate in map's players location and disable input for them. Players are ready, so tell camera to start working, create UI widget and Fade In
      (`self.GetGameCameraRef`))
    (:`then_1`
      (`GameplayStatics.CreatePlayer` -1)
      (bind _asikabomb_ginstance_bp (cast `/Game/Blueprint/IKABombGInstanceBP` (`GameplayStatics.GetGameInstance`)))
      (`KismetArrayLibrary.Array_Set` _playersclass 0 (`/Game/Blueprint/IKABombGInstanceBP.Player1Class` _asikabomb_ginstance_bp))
      (`KismetArrayLibrary.Array_Set` _playersclass 1 (`/Game/Blueprint/IKABombGInstanceBP.Player2Class` _asikabomb_ginstance_bp)))
    (:`then_2`
      (for _index (range 2)
        (bind _returnvalue (`IKAMapManager.GetPlayerStartLocation` (`self.MapReference`) _index))
        (bind _returnvalue_2 (`|SpawnActorFromClass` (`|GetArrayItem` (`self.PlayersClass`) _index) (`KismetMathLibrary.MakeTransform` (+ _returnvalue (0.0 0.0 50.0))) "Undefined" "OverrideRootScale" null null))
        (`Controller.Possess` (`GameplayStatics.GetPlayerController` _index) _returnvalue_2)
        (bind _asikaplayer (cast `IKAPlayer` _returnvalue_2))
        (`KismetArrayLibrary.Array_Add` (`self.CurrentPlayers`) _asikaplayer)
        (`IKAPlayer.SetPlayerInputEnabled` _asikaplayer false)))
    (:`then_3`
      (`IKAGameCamera.StartWorking` (`self.GameCameraRef`)))
    (:`then_4`
      (bind _returnvalue_3 (`|CreateWidget` "/Game/UI/UIGame_W.UIGame_W_C"))
      (bind _output_get (set `self.GameUI` _returnvalue_3))
      (`UserWidget.AddToViewport` _output_get 0))
    (:`then_5`
      (`KismetSystemLibrary.Delay` 1.0)
      (`PlayerCameraManager.StartCameraFade` (`GameplayStatics.GetPlayerCameraManager` 0) 1.0 0.0 2.0 (struct :`R` 1.0 :`G` 1.0 :`B` 1.0 :`A` 1.0) false false))
    (:`then_6`
      (`self.GetReferences`)
      (set `PlayerController.bShowMouseCursor` false (`GameplayStatics.GetPlayerController` 0))
      (`WidgetBlueprintLibrary.SetFocusToGameViewport`))))

(event `self.ReadyMessage`
  ;[1 1 1] Show "Ready" and "Start" UI messages
  (`parent.ReadyMessage`)
  (`/Engine/EditorBlueprintResources/StandardMacros.IsValid` (`self.GameUI`)
    (:`Is Valid`
      (`/Game/UI/UIGame_W.SetMessage` (`self.GameUI`) "Ready" 1.0))))

(event `self.GameStarted`
  (bind _gameui (`self.GameUI`))
  ;[1 1 1] Show "Ready" and "Start" UI messages
  (`parent.GameStarted`)
  (`/Engine/EditorBlueprintResources/StandardMacros.IsValid` (`self.GameUI`)
    (:`Is Valid`
      (`/Game/UI/UIGame_W.SetMessage` _gameui "Start!" 1.0)
      (`/Game/UI/UIGame_W.StartTimeCount` _gameui)
      (`self.EnablePlayersInput` true))))

(event `self.TimeOver`
  ;[1 1 1] Time Over Event
  (`self.CheckEndGameConditions`))

(event `self.PlayerDeadBy`
  (params (PlayerId :type Integer) (DeathCauser :type "Actor Object Reference"))
  ;[1 1 1] When a player die, wait to check if both are dead or just one, to check who won
  (`BlueprintMapLibrary.Map_Add` (`self.PlayersDeath`) PlayerId DeathCauser)
  (if (not (`KismetSystemLibrary.K2_IsTimerActiveHandle` (`self.EndConditionsTimer`)))
    (bind _returnvalue (`KismetSystemLibrary.K2_SetTimer` self "CheckEndGameConditions" 0.5))
    (set `self.EndConditionsTimer` _returnvalue)
    (set `self.FirstPlayerDead` PlayerId)))

(fn `CheckEndGameConditions`
  (`KismetSystemLibrary.K2_ClearAndInvalidateTimerHandle` (`self.GameTimerHandle`))
  (`/Game/UI/UIGame_W.StopTimeCount` (`self.GameUI`))
  (`self.EnablePlayersInput` false)
  (if (or (and (== (`KismetArrayLibrary.Array_Length` (`self.CurrentPlayers`)) (`BlueprintMapLibrary.Map_Length` (`self.PlayersDeath`))) (`self.SameDamageCauser`)) (< (`self.FirstPlayerDead`) 0))
    ;[1 1 1] Draw Game
    (`/Game/UI/UIGame_W.SetMessage` (`self.GameUI`) "Draw!!" 3.0)
    (`KismetSystemLibrary.K2_SetTimer` self "ShowEndGameMenu" 4.0)
    (`self.SaveGame` "NewEnumerator2")
    (`self.SetGameplayState` "EFinished")
    (else
      ;[1 1 1] Search the winner, show a message and trigger state for animations
      (for (_array_element _array_index) (`self.CurrentPlayers`)
        (if (!= _array_index (`self.FirstPlayerDead`))
          (`/Game/UI/UIGame_W.SetMessage` (`self.GameUI`) (`KismetTextLibrary.Conv_StringToText` (`KismetStringLibrary.Concat_StrStr` "Player " (`KismetStringLibrary.Conv_IntToString` (+ _array_index 1)) " Wins!!")) 3.0)
          (`IKAPlayer.SetPlayerWinner` _array_element)
          (`self.SaveGame` (cast `/Game/Data/GameWinner` (`KismetMathLibrary.Conv_IntToByte` _array_index)))
          (`AudioComponent.FadeOut` (`AmbientSound.AudioComponent` (`self.LevelMusic`)) 3.0 0.0)
          (`GameplayStatics.PlaySound2D` "/Game/Sound/fanfare_Cue.fanfare_Cue")))
      ;[1 1 1] Show delayed menu
      (`KismetSystemLibrary.K2_SetTimer` self "ShowEndGameMenu" 4.0)
      (`self.SetGameplayState` "EFinished"))))

(fn `EnablePlayersInput`
  (params (enable :type Boolean))
  (for _array_element (`self.CurrentPlayers`)
    (`IKAPlayer.SetPlayerInputEnabled` _array_element enable)))

(fn `ExitGame`
  (params (restart :type Boolean))
  (for _index (range (- (`KismetArrayLibrary.Array_Length` (`self.CurrentPlayers`)) 1) 2)
    (`GameplayStatics.RemovePlayer` (`GameplayStatics.GetPlayerController` _index) true))
  (bind _asikabomb_ginstance_bp (cast `/Game/Blueprint/IKABombGInstanceBP` (`GameplayStatics.GetGameInstance`)))
  (`/Game/Blueprint/IKABombGInstanceBP.RestartGame` _asikabomb_ginstance_bp restart))

(fn `GetGameCameraRef`
  (bind _outactors (`GameplayStatics.GetAllActorsOfClass` "/Script/IKABombermanUE.IKAGameCamera"))
  (if (== (`KismetArrayLibrary.Array_Length` _outactors) 0)
    (bind _returnvalue (`|SpawnActorFromClass` "/Game/Blueprint/GameCameraBP.GameCameraBP_C" (`KismetMathLibrary.MakeTransform` (0.0 0.0 0.0) (`KismetMathLibrary.MakeRotator` 0.0 (`self.DefaultCameraPitchRot`))) "Undefined" "OverrideRootScale" null null))
    (set `self.GameCameraRef` _returnvalue)
    (else
      (set `self.GameCameraRef` (`|GetArrayItem` _outactors)))))

(fn `GetReferences`
  (`|ExecutionSequence`
    (:`then_0`
      (bind _outactors (`GameplayStatics.GetAllActorsOfClass` "/Script/Engine.DirectionalLight"))
      (set `self.LightSource` (`|GetArrayItem` _outactors)))
    (:`then_1`
      (bind _outactors_2 (`GameplayStatics.GetAllActorsOfClass` "/Script/Engine.PostProcessVolume"))
      (set `self.PPRef` (`|GetArrayItem` _outactors_2)))
    (:`then_2`
      (bind _outactors_3 (`GameplayStatics.GetAllActorsOfClass` "/Script/Engine.SkyLight"))
      (set `self.SkyLightRef` (`|GetArrayItem` _outactors_3)))
    (:`then_3`
      (bind _outactors_4 (`GameplayStatics.GetAllActorsOfClass` "/Script/Engine.AmbientSound"))
      (set `self.LevelMusic` (`|GetArrayItem` _outactors_4)))))

(fn `SameDamageCauser`
  (returns (return :type Boolean))
  (locals (DeathCauser :type "Actor Object Reference") (same :type Boolean :default true))
  ;[1 1 1] Check if all the death causer are the same
  (set `local.DeathCauser` (`BlueprintMapLibrary.Map_Find` (`self.PlayersDeath`)))
  (for _index (range 1 (`KismetArrayLibrary.Array_Length` (`self.CurrentPlayers`)))
    (if (!= (`local.DeathCauser`) (`BlueprintMapLibrary.Map_Find` (`self.PlayersDeath`) _index))
      (set `local.same` false)
      (else
        (break))))
  (return (`local.same`)))

(fn `SaveGame`
  (params (winner :type "/Game/Data/GameWinner Enum" :default "NewEnumerator0"))
  (bind _asikabomb_ginstance_bp (cast `/Game/Blueprint/IKABombGInstanceBP` (`GameplayStatics.GetGameInstance`)))
  (`/Game/Blueprint/IKABombGInstanceBP.SaveGameData` _asikabomb_ginstance_bp (make `/Game/Data/GamesData` (`KismetMathLibrary.Now`) winner)))

(fn `ShowEndGameMenu`
  (bind _returnvalue (`|CreateWidget` "/Game/UI/UIEndGame_W.UIEndGame_W_C"))
  (`UserWidget.AddToViewport` _returnvalue 0)
  (set `PlayerController.bShowMouseCursor` true (`GameplayStatics.GetPlayerController` 0)))

(fn `TurnOffLights`
  (params (time :type "Float (double-precision)"))
  (bind _ppref (`self.PPRef`))
  (bind _skylightref (`self.SkyLightRef`))
  (bind _lightsource (`self.LightSource`))
  (`|ExecutionSequence`
    (:`then_0`
      (`/Engine/EditorBlueprintResources/StandardMacros.IsValid` _lightsource
        (:`Is Valid`
          (`SceneComponent.SetVisibility` (`Light.LightComponent` _lightsource) false false))))
    (:`then_1`
      (`/Engine/EditorBlueprintResources/StandardMacros.IsValid` _ppref
        (:`Is Valid`
          (set `PostProcessVolume.bEnabled` false _ppref))))
    (:`then_2`
      (`/Engine/EditorBlueprintResources/StandardMacros.IsValid` _skylightref
        (:`Is Valid`
          (`SceneComponent.SetVisibility` (`SkyLight.LightComponent` _skylightref) false false))))
    (:`then_3`
      (`KismetSystemLibrary.K2_SetTimer` self "TurnOn" time))))

(fn `TurnOn`
  (bind _ppref (`self.PPRef`))
  (bind _skylightref (`self.SkyLightRef`))
  (bind _lightsource (`self.LightSource`))
  (`|ExecutionSequence`
    (:`then_0`
      (`/Engine/EditorBlueprintResources/StandardMacros.IsValid` _lightsource
        (:`Is Valid`
          (`SceneComponent.SetVisibility` (`Light.LightComponent` _lightsource) true true))))
    (:`then_1`
      (`/Engine/EditorBlueprintResources/StandardMacros.IsValid` _ppref
        (:`Is Valid`
          (set `PostProcessVolume.bEnabled` true _ppref))))
    (:`then_2`
      (`/Engine/EditorBlueprintResources/StandardMacros.IsValid` _skylightref
        (:`Is Valid`
          (`SceneComponent.SetVisibility` (`SkyLight.LightComponent` _skylightref) true true))))))

(fn `UserConstructionScript`)