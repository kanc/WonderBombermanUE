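; Game mode for the menu that shows a randomly chosen backdrop view when play begins.
; On BeginPlay it fades the screen to white and holds it while blending the player's view to a random actor tagged MenuCamera.
; After a one-second delay it fades back in from white, so the camera switch is hidden behind the fade.
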(event `self.ReceiveBeginPlay`
  (`PlayerCameraManager.StartCameraFade` (`GameplayStatics.GetPlayerCameraManager` 0) 0.0 1.0 0.1 (struct :`R` 1.0 :`G` 1.0 :`B` 1.0 :`A` 1.0) false true)
  (bind _outactors (`GameplayStatics.GetAllActorsWithTag` "MenuCamera"))
  (`PlayerController.SetViewTargetWithBlend` (`GameplayStatics.GetPlayerController` 0) (`|GetArrayItem` _outactors (`KismetMathLibrary.RandomIntegerInRange` 0 (- (`KismetArrayLibrary.Array_Length` _outactors) 1))) 1.0 "VTBlend_Linear" 0.0 false)
  (`KismetSystemLibrary.Delay` 1.0)
  (`PlayerCameraManager.StartCameraFade` (`GameplayStatics.GetPlayerCameraManager` 0) 1.0 0.0 1.0 (struct :`R` 1.0 :`G` 1.0 :`B` 1.0 :`A` 1.0) false false))

(fn `UserConstructionScript`)