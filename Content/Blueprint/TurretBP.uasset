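; Turret that periodically picks a random player, tracks them with its cannon and fires a projectile.
; Chained timers alternate a random wait, target selection and a timed tracking window that ends in the shot.
; While targeting, Tick smoothly turns only the cannon's yaw toward the target.
; Shots fire and reschedule only during the Playing state, adding sound, particles and an off-screen UI indicator for each projectile.
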(event `self.ReceiveBeginPlay`
  (bind (_x _y) (`KismetMathLibrary.BreakVector2D` (`self.TimeToShot`)))
  (`KismetSystemLibrary.Delay` 1.0)
  (`|ExecutionSequence`
    (:`then_0`
      (bind _foundwidgets (`WidgetBlueprintLibrary.GetAllWidgetsOfClass` "/Game/UI/UIGame_W.UIGame_W_C"))
      (if (> (`KismetArrayLibrary.Array_Length` _foundwidgets) 0)
        (bind _output_get (set `self.UIRef` (`|GetArrayItem` _foundwidgets)))
        (set `/Game/UI/UIGame_W.OffScreenIndicators` true _output_get)))
    (:`then_1`
      (bind _asikagame_mode_base (cast `IKAGameModeBase` (`GameplayStatics.GetGameMode`)))
      (set `self.Players` (`IKAGameModeBase.CurrentPlayers` _asikagame_mode_base))
      (set `self.Targeting` true)
      (`KismetSystemLibrary.K2_SetTimer` self "GetTarget" (`KismetMathLibrary.RandomFloatInRange` _x _y)))))

(event `self.ReceiveTick`
  (params (DeltaSeconds :type "Float (single-precision)"))
  (if (`self.Targeting`)
    (`self.FollowTarget`)))

(fn `FollowTarget`
  (locals (Position :type "Vector Structure"))
  (bind _currenttarget (`self.currentTarget`))
  (bind _returnvalue (`SceneComponent.K2_GetComponentRotation` (`self.Canon`)))
  (bind (_returnvalue_roll _returnvalue_pitch _returnvalue_yaw) (`KismetMathLibrary.BreakRotator` (`KismetMathLibrary.RInterpTo` _returnvalue (`KismetMathLibrary.FindLookAtRotation` (`SceneComponent.K2_GetComponentLocation` (`self.Canon`)) (`local.Position`)) (`GameplayStatics.GetWorldDeltaSeconds`) (`self.TargetingSpeed`))))
  (`/Engine/EditorBlueprintResources/StandardMacros.IsValid` _currenttarget
    (:`Is Valid`
      (set `local.Position` (`self.K2_GetActorLocation` _currenttarget)))
    (:`Is Not Valid`
      (set `local.Position` (0.0 0.0 0.0))))
  (`SceneComponent.K2_SetWorldRotation` (`self.Canon`) (`KismetMathLibrary.MakeRotator` (.roll _returnvalue) (.pitch _returnvalue) _returnvalue_yaw) false false))

(fn `GetTarget`
  (bind _players (`self.Players`))
  (set `self.currentTarget` (`|GetArrayItem` _players (`KismetMathLibrary.RandomIntegerInRange` 0 (- (`KismetArrayLibrary.Array_Length` _players) 1))))
  (set `self.Targeting` true)
  (`KismetSystemLibrary.K2_SetTimer` self "StopTargeting" (`self.TimeTargeting`)))

(fn `Shot`
  (bind (_x _y) (`KismetMathLibrary.BreakVector2D` (`self.TimeToShot`)))
  (bind _asikagame_mode_base (cast `IKAGameModeBase` (`GameplayStatics.GetGameMode`)))
  (bind _returnvalue (`IKAGameModeBase.GetGameplayState` _asikagame_mode_base))
  (if (`|EnumEquality` _returnvalue "EPlaying")
    (bind _returnvalue_2 (`|SpawnActorFromClass` (`self.ProjectileBP`) (`KismetMathLibrary.MakeTransform` (`SceneComponent.K2_GetComponentLocation` (`self.ShotPoint`))) "Undefined" "OverrideRootScale" null (`SceneComponent.GetForwardVector` (`self.ShotPoint`)) null))
    (`GameplayStatics.PlaySoundAtLocation` "/Game/Sound/TurretShot_S.TurretShot_S" (`self.K2_GetActorLocation`))
    (`ActorComponent.SetActive` (`self.ParticleSystem`) true true)
    (`KismetSystemLibrary.K2_SetTimer` self "GetTarget" (`KismetMathLibrary.RandomFloatInRange` _x _y))
    (`/Engine/EditorBlueprintResources/StandardMacros.IsValid` (`self.UIRef`)
      (:`Is Valid`
        (`/Game/UI/UIGame_W.AddOffScreenIndicator` (`self.UIRef`) _returnvalue_2)))))

(fn `StopTargeting`
  (set `self.Targeting` false)
  (`self.Shot`))

(fn `UserConstructionScript`)