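; Two-player character selection actor that gives each player a camera and a clamped index into the PlayerClasses map.
; Selection changes shift that player's camera target sideways along Y by a fixed increment per step.
; Tick eases each moving camera toward its target with VInterpTo, then snaps it in place within a small tolerance.
; SetPlayerClasses writes both chosen classes to IKABombGInstanceBP, the game instance.
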(event `self.ReceiveBeginPlay`
  (set `self.P1CameraTarget` (`SceneComponent.RelativeLocation` (`self.CameraP1`)))
  (set `self.P2CameraTarget` (`SceneComponent.RelativeLocation` (`self.CameraP2`))))

(event `self.ReceiveTick`
  (params (DeltaSeconds :type "Float (single-precision)"))
  (`|ExecutionSequence`
    (:`then_0`
      (if (`self.P1Moving`)
        (bind _finish (`self.MoveCameraTo` (`self.CameraP1`) (`self.P1CameraTarget`)))
        (bind _output_get (set `self.P1Moving` (not _finish)))
        (if (not _output_get)
          (`SceneComponent.K2_SetRelativeLocation` (`self.CameraP1`) (`self.P1CameraTarget`) false true))))
    (:`then_1`
      (if (`self.P2Moving`)
        (bind _finish_2 (`self.MoveCameraTo` (`self.CameraP2`) (`self.P2CameraTarget`)))
        (bind _output_get_2 (set `self.P2Moving` (not _finish_2)))
        (if (not _output_get_2)
          (`SceneComponent.K2_SetRelativeLocation` (`self.CameraP2`) (`self.P2CameraTarget`) false true))))))

(fn `GetPlayerClass`
  (params (playerid :type Integer))
  (returns (class :type "IKAPlayer Class Reference"))
  (bind _playerclasses (`self.PlayerClasses`))
  (switch `int` playerid
    (:`Default`
      (return (`BlueprintMapLibrary.Map_Find` _playerclasses)))
    (:`0`
      (return (`BlueprintMapLibrary.Map_Find` _playerclasses (`self.P1Index`))))
    (:`1`
      (return (`BlueprintMapLibrary.Map_Find` _playerclasses (`self.P2Index`))))))

(fn `MoveCameraTo`
  (params (camera :type "CameraComponent Object Reference") (To :type "Vector Structure"))
  (returns (finish :type Boolean))
  (bind _relativelocation (`SceneComponent.RelativeLocation` camera))
  (`SceneComponent.K2_SetRelativeLocation` camera (`KismetMathLibrary.VInterpTo` _relativelocation To (`GameplayStatics.GetWorldDeltaSeconds`) 10.0) false false)
  (return (== _relativelocation To :`ErrorTolerance` 0.2)))

(fn `P1SelectionChange`
  (params (movement :type Integer))
  (locals (tempIndex :type Integer))
  (set `local.tempIndex` (`KismetMathLibrary.Clamp` (+ movement (`self.P1Index`)) 0 (- (`BlueprintMapLibrary.Map_Length` (`self.PlayerClasses`)) 1)))
  (if (!= (`local.tempIndex`) (`self.P1Index`))
    (set `self.P1CameraTarget` (+ (`self.P1CameraTarget`) (`KismetMathLibrary.MakeVector` 0.0 (* movement (`self.MovIncrement`)))))
    (set `self.P1Moving` true)
    (set `self.P1Index` (`local.tempIndex`))))

(fn `P2SelectionChange`
  (params (movement :type Integer))
  (locals (tempIndex :type Integer))
  (set `local.tempIndex` (`KismetMathLibrary.Clamp` (+ movement (`self.P2Index`)) 0 (- (`BlueprintMapLibrary.Map_Length` (`self.PlayerClasses`)) 1)))
  (if (!= (`local.tempIndex`) (`self.P2Index`))
    (set `self.P2CameraTarget` (+ (`self.P2CameraTarget`) (`KismetMathLibrary.MakeVector` 0.0 (* movement (`self.MovIncrement`)))))
    (set `self.P2Moving` true)
    (set `self.P2Index` (`local.tempIndex`))))

(fn `SetPlayerClasses`
  (bind _asikabomb_ginstance_bp (cast `/Game/Blueprint/IKABombGInstanceBP` (`GameplayStatics.GetGameInstance`)))
  (`|ExecutionSequence`
    (:`then_0`
      (bind _class (`self.GetPlayerClass` 0))
      (set `/Game/Blueprint/IKABombGInstanceBP.Player1Class` _class _asikabomb_ginstance_bp))
    (:`then_1`
      (bind _class_2 (`self.GetPlayerClass` 1))
      (set `/Game/Blueprint/IKABombGInstanceBP.Player2Class` _class_2 _asikabomb_ginstance_bp))))

(fn `UserConstructionScript`)